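; BP_VehiclePawn is a vehicle pawn Blueprint whose graph handles toggling the in-game pause menu.
; The IA_Pause Enhanced Input action flips a flag to open or close the WB_PauseMenu widget.
; Opening creates a fresh widget, pauses the game, shows the cursor and uses Game and UI input.
; Closing removes the widget, unpauses, hides the cursor and restores game-only input.
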(event `EnhancedInput|/Game/ProjectA/Core/Input/Actions/IA_Pause`
  (params (ActionValue :type Boolean) (ElapsedSeconds :type "Float (double-precision)") (TriggeredSeconds :type "Float (double-precision)") (InputAction :type "InputAction Object Reference" :default "/Game/ProjectA/Core/Input/Actions/IA_Pause.IA_Pause"))
  (bind _returnvalue (`GameplayStatics.GetPlayerController` 0))
  (:`Started`
    (if (not (`self.bIsPauseMenuOpened`))
      (set `self.bIsPauseMenuOpened` true)
      (bind _returnvalue_2 (`|CreateWidget` "/Game/ProjectA/Core/UI/WB_PauseMenu.WB_PauseMenu_C"))
      (bind _output_get (set `self.PauseMenuWidget` _returnvalue_2))
      (`UserWidget.AddToViewport` _output_get 0)
      (`WidgetBlueprintLibrary.SetInputMode_GameAndUIEx` _returnvalue null)
      (set `PlayerController.bShowMouseCursor` true _returnvalue)
      (`GameplayStatics.SetGamePaused` true)
      (else
        (set `self.bIsPauseMenuOpened` false)
        (`Widget.RemoveFromParent` (`self.PauseMenuWidget`))
        (`GameplayStatics.SetGamePaused` false)
        (`WidgetBlueprintLibrary.SetInputMode_GameOnly` _returnvalue)
        (set `PlayerController.bShowMouseCursor` false _returnvalue)))))

(fn `UserConstructionScript`)